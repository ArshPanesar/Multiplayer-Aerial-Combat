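; BP_ACPlayerController is the player controller that sets up the HUD, handles respawns and feeds the leaderboard.
; BeginPlay assigns BP_HUD, and RespawnPlayer asks BP_ACGameModeBase to destroy the player, then respawn them after a short delay.
; UpdatePlayerListOnClient sorts the player stats by kills, descending, with a nested-loop swap sort and passes them to the HUD widget.
; The construction script holds unconnected windowed-resolution setup that never runs.
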(event Custom|RespawnPlayer
  (bind _asbp_acgame_mode_base (Utilities|Casting|CastToBP_ACGameModeBase (Game|GetGameMode)))
  (Default|DestroyPlayer _asbp_acgame_mode_base self)
  (Utilities|FlowControl|Delay 0.2)
  (Default|RespawnRequested _asbp_acgame_mode_base self)
  (Utilities|FlowControl|Delay 0.2))

(event Custom|UpdatePlayerListOnClient
  (params (PlayerList :type Array%20of%20S%20Player%20Stats%20Structures))
  (bind _asbp_hud (Utilities|Casting|CastToBP_HUD (HUD|GetHUD)))
  (Utilities|IsValid (Variables|/Game/Blueprints/BP_HUD.BP_HUD_C|GetHUD_Ref _asbp_hud)
    (:Is%20Valid
      (bind _sortedplayerlist (CallFunction|SortPlayerStatsList PlayerList))
      (Default|UpdateLeaderboard (Variables|/Game/Blueprints/BP_HUD.BP_HUD_C|GetHUD_Ref _asbp_hud) _sortedplayerlist))))

(event EventBeginPlay
  (Class|PlayerController|ClientSetHUD "/Game/Blueprints/BP_HUD.BP_HUD_C"))

(event EventTick
  (params (DeltaSeconds :type Float%20%28single-precision%29)))

(fn ConstructionScript)

(fn SortPlayerStatsList
  (params (PlayerList :type Array%20of%20S%20Player%20Stats%20Structures))
  (for (_ _array_index) PlayerList
    (bind _output_get (LocalVariables|SetOuterItr _array_index))
    (bind _index (Utilities|FlowControl|ForLoopwithBreak (+ _output_get 1) (- (Utilities|Array|Length PlayerList) 1))
      (:LoopBody
        (bind _output_get_2 (LocalVariables|SetInnerItr _index))
        (if (> (.Kills (Utilities|Struct|BreakS_PlayerStats (Utilities|Array|Get(acopy) PlayerList _output_get_2))) (.Kills (Utilities|Struct|BreakS_PlayerStats (Utilities|Array|Get(acopy) PlayerList (LocalVariables|GetOuterItr)))))
          (Utilities|Array|Swap PlayerList (LocalVariables|GetOuterItr) (LocalVariables|GetInnerItr))))))
  (return PlayerList))