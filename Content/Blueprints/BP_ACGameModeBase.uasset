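; Game mode for a multiplayer vehicle combat game that handles vehicle respawning and the shared player scoreboard.
; Authority-only events destroy a player's pawn or spawn a BP_CombatVehicle at a start found using player 0, then possess it after a short delay.
; Logins and logouts maintain a controller list.
; These changes and respawns rebuild name, kill and death stats, which are pushed to every player controller.
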(event Custom|RespawnRequested
  (params (Player%20Controller :type AC%20Player%20Controller%20Object%20Reference))
  (Utilities|IsValid Player%20Controller
    (:Is%20Valid
      (Networking|SwitchHasAuthority
        (:Authority
          (bind _returnvalue (Game|SpawnActorfromClass "/Game/Blueprints/BP_CombatVehicle.BP_CombatVehicle_C" (Transformation|GetActorTransform (Class|GameModeBase|FindPlayerStart (Game|GetPlayerController 0))) "Undefined" "MultiplyWithRoot" 0 0))
          (Utilities|FlowControl|Delay 0.2)
          (Pawn|Possess Player%20Controller _returnvalue)
          (CallFunction|UpdatePlayerList))))))

(event Custom|DestroyPlayer
  (params (PlayerController :type AC%20Player%20Controller%20Object%20Reference))
  (Utilities|IsValid PlayerController
    (:Is%20Valid
      (Networking|SwitchHasAuthority
        (:Authority
          (Actor|DestroyActor (Pawn|GetControlledPawn PlayerController)))))))

(event EventBeginPlay)

(event EventTick
  (params (DeltaSeconds :type Float%20%28single-precision%29)))

(event EventPostLogin
  (params (NewPlayer :type Player%20Controller%20Object%20Reference))
  (Utilities|Array|Add (Variables|Default|GetAllPlayerControllers) NewPlayer)
  (Utilities|FlowControl|Delay 0.2)
  (CallFunction|UpdatePlayerList))

(event EventOnLogout
  (params (ExitingController :type Controller%20Object%20Reference))
  (bind _asplayer_controller (Utilities|Casting|CastToPlayerController ExitingController))
  (Utilities|Array|RemoveItem (Variables|Default|GetAllPlayerControllers) _asplayer_controller)
  (Utilities|FlowControl|Delay 0.2)
  (CallFunction|UpdatePlayerList))

(fn ConstructionScript)

(fn UpdatePlayerList
  (Utilities|Array|Clear (Variables|Default|GetAllPlayerStats))
  (for _array_element (Variables|Default|GetAllPlayerControllers)
    (Utilities|FlowControl|Sequence
      (:then_0
        (bind _asbp_acplayer_controller (Utilities|Casting|CastToBP_ACPlayerController _array_element)))
      (:then_1
        (bind _asbp_acplayer_state (Utilities|Casting|CastToBP_ACPlayerState (Variables|/Script/Engine.Controller|GetPlayerState _array_element))))
      (:then_2
        (Utilities|Array|Add (Variables|Default|GetAllPlayerStats) (Utilities|Struct|MakeS_PlayerStats (Variables|/Game/Blueprints/BP_ACPlayerController.BP_ACPlayerController_C|GetPlayerNameTag _asbp_acplayer_controller) (Variables|/Script/AerialCombat.ACPlayerState|GetNumKills _asbp_acplayer_state) (Variables|/Script/AerialCombat.ACPlayerState|GetNumDeaths _asbp_acplayer_state))))))
  (for _array_element_2 (Variables|Default|GetAllPlayerControllers)
    (bind _asbp_acplayer_controller_2 (Utilities|Casting|CastToBP_ACPlayerController _array_element_2))
    (Default|UpdatePlayerListonClient _asbp_acplayer_controller_2 (Variables|Default|GetAllPlayerStats))))