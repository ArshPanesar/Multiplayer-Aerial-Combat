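; BP_CombatVehicle is a networked player combat vehicle that handles name tags, HUD feedback and death.
; The owning client sends its GameInstance player name to the server, and OnRep updates the tag widget, with timers retrying until ready; other players' tags face the camera.
; Health and lock-in events forward to the HUD.
; Death multicasts hiding the mesh and spawning an exploded vehicle, while the authority asks the controller to respawn after a delay.
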(event Custom|Respawn
  (bind _asbp_acplayer_controller (Utilities|Casting|CastToBP_ACPlayerController (Pawn|GetController)))
  (Default|RespawnPlayer _asbp_acplayer_controller))

(event Custom|RPC_Multicast_Death
  (Rendering|SetVisibility (Variables|Default|GetStaticMesh) false true)
  (Game|SpawnActorfromClass "/Game/Blueprints/BP_GC_ExplodedCombatVehicle.BP_GC_ExplodedCombatVehicle_C" (Transformation|GetActorTransform) "AlwaysSpawn" "MultiplyWithRoot" 0 0))

(event Custom|RPC_Server_SetNameTag
  (params (NameTag :type Text))
  (Variables|Default|SetNameTag NameTag))

(event EventBeginPlay
  (CallFunction|SetNameTag))

(event Collision|EventActorBeginOverlap
  (params (OtherActor :type Actor%20Object%20Reference)))

(event EventTick
  (params (DeltaSeconds :type Float%20%28single-precision%29))
  (CallFunction|UpdateNameTagFaceCamera))

(event EventUIonHealthUpdate
  (params (Health :type Float%20%28single-precision%29))
  (bind _asbp_hud (Utilities|Casting|CastToBP_HUD (HUD|GetHUD (Game|GetPlayerController 0))))
  (Default|OnHealthUpdate (Variables|/Game/Blueprints/BP_HUD.BP_HUD_C|GetHUD_Ref _asbp_hud) Health))

(event EventUISetLockedin
  (params (bActivate :type Boolean))
  (bind _asbp_hud (Utilities|Casting|CastToBP_HUD (HUD|GetHUD (Game|GetPlayerController 0))))
  (Default|SetLockedin (Variables|/Game/Blueprints/BP_HUD.BP_HUD_C|GetHUD_Ref _asbp_hud) bActivate))

(event EventPlayerDeath
  (Utilities|FlowControl|Sequence
    (:then_0
      (Networking|SwitchHasAuthority
        (:Authority
          (Utilities|Time|SetTimerbyEvent (delegate Custom|Respawn) 1.0))))
    (:then_1
      (CallFunction|RPCMulticastDeath))))

(fn ConstructionScript)

(fn SetNameTag
  (if (Pawn|IsLocallyControlled)
    (bind _asbp_acgame_instance (Utilities|Casting|CastToBP_ACGameInstance (Game|GetGameInstance)))
    (CallFunction|RPCServerSetNameTag (Variables|/Game/Blueprints/BP_ACGameInstance.BP_ACGameInstance_C|GetPlayerName _asbp_acgame_instance))
    (else
      (Utilities|Time|SetTimerbyFunctionName 0 "SetNameTag" 0.1))))

(fn OnRepNameTag
  (bind _w_playernametag (Variables|Default|GetW_PlayerNameTag))
  (bind _returnvalue (UserInterface|GetWidget _w_playernametag))
  (Utilities|IsValid _returnvalue
    (:Is%20Valid
      (bind _aswb_player_name_tag (Utilities|Casting|CastToWB_PlayerNameTag _returnvalue))
      (Default|SetPlayerName _aswb_player_name_tag (Variables|Default|GetNameTag)))
    (:Is%20Not%20Valid
      (Utilities|Time|SetTimerbyFunctionName 0 "OnRep_NameTag" 0.1))))

(fn UpdateNameTagFaceCamera
  (if (not (Pawn|IsLocallyControlled))
    (Transformation|SetWorldRotation (Variables|Default|GetW_PlayerNameTag) (Math|Rotator|FindLookatRotation (Transformation|GetWorldLocation (Variables|Default|GetW_PlayerNameTag)) (Transformation|GetActorLocation (Game|GetPlayerCameraManager 0))) false false)))